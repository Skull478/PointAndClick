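; Interactive light actor, a child of a base interactive actor, that toggles on and off each time it is interacted with.
; It starts on, and Interact flips IsOn to swap the mesh between glow and no-glow materials and show or hide the point light.
; The construction script places the light and a Switch component relative to the mesh from offset variables.
; The Switch is hidden at BeginPlay.
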(event EventBeginPlay
  (|CallParentFunction)
  (Variables|Default|SetisOn? true)
  (Rendering|SetVisibility (Variables|Default|GetSwitch) false false)
  (Rendering|Material|SetMaterial (Variables|Default|GetStaticMesh) 0 "/Game/DetectiveStart/Assets/Materials/M_Glow.M_Glow")
  (Rendering|SetVisibility (Variables|Default|GetPointLight) true false))

(event EventInteract
  (bind _staticmesh (Variables|Default|GetStaticMesh))
  (bind _pointlight (Variables|Default|GetPointLight))
  (|CallParentFunction)
  (bind _output_get (Variables|Default|SetisOn? (not (Variables|Default|GetisOn?))))
  (if _output_get
    (Rendering|Material|SetMaterial _staticmesh 0 "/Game/DetectiveStart/Assets/Materials/M_Glow.M_Glow")
    (Rendering|SetVisibility _pointlight true false)
    (else
      (Rendering|Material|SetMaterial _staticmesh 0 "/Game/DetectiveStart/Assets/Materials/M_NoGlow.M_NoGlow")
      (Rendering|SetVisibility _pointlight false false))))

(fn ConstructionScript
  (bind _switch_scale (Variables|Default|GetSwitch_Scale))
  (bind _staticmesh (Variables|Default|GetStaticMesh))
  (|CallParentFunction)
  (Transformation|SetWorldLocation (Variables|Default|GetPointLight) (+ (Transformation|GetWorldLocation _staticmesh) (Variables|Default|GetLight_Offset)) false false)
  (Transformation|SetWorldTransform (Variables|Default|GetSwitch) (Math|Transform|MakeTransform (+ (Transformation|GetWorldLocation _staticmesh) (Variables|Default|GetSwitch_Position)) (Variables|Default|GetSwitch_Rotation) (* (Transformation|GetWorldScale (Variables|Default|GetSwitch)) (Math|Vector|MakeVector _switch_scale _switch_scale _switch_scale))) false false))

(fn GetInfos
  (params (ObjectName :type Name :default "None"))
  (return ""))