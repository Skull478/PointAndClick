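; An interactive desk lamp actor, built on a base interactive actor, that the player can switch on and off.
; Interact flips an IsOn flag and plays or reverses the Off timeline, whose Luminosity track drives the point light's intensity.
; BeginPlay sets the lamp as on and calls reverse on that timeline.
; Overlapping the sphere shows a widget, and leaving it hides the widget.
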(event OnComponentBeginOverlap(Sphere)
  (params (OverlappedComponent :type Primitive%20Component%20Object%20Reference) (OtherActor :type Actor%20Object%20Reference) (OtherComp :type Primitive%20Component%20Object%20Reference) (OtherBodyIndex :type Integer) (bFromSweep :type Boolean) (SweepResult :type Hit%20Result%20Structure%20%28by%20ref%29))
  (Rendering|SetVisibility (Variables|Default|GetWidget) true false))

(event OnComponentEndOverlap(Sphere)
  (params (OverlappedComponent :type Primitive%20Component%20Object%20Reference) (OtherActor :type Actor%20Object%20Reference) (OtherComp :type Primitive%20Component%20Object%20Reference) (OtherBodyIndex :type Integer))
  (Rendering|SetVisibility (Variables|Default|GetWidget) false false))

(event EventBeginPlay
  (|CallParentFunction)
  (Variables|Default|SetisOn? true)
  (bind _luminosity (Timeline|Off Reverse)
    (:Update
      (Rendering|Components|Light|SetIntensity (Variables|Default|GetPointLight) _luminosity))))

(event EventInteract
  (|CallParentFunction)
  (bind _output_get (Variables|Default|SetisOn? (not (Variables|Default|GetisOn?))))
  (if _output_get
    (bind _luminosity (Timeline|Off Reverse)
      (:Update
        (Rendering|Components|Light|SetIntensity (Variables|Default|GetPointLight) _luminosity)))
    (else
      (Timeline|Off Play))))

(fn ConstructionScript
  (|CallParentFunction))