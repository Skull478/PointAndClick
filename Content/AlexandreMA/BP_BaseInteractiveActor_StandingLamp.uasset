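; Standing lamp interactive actor that toggles its spotlight on and off when interacted with.
; It extends a base interactive actor, calling the parent BeginPlay and Interact before its own logic.
; An IsOn flag starts true and flips on each interaction, choosing the direction of a single Off timeline.
; The timeline plays to switch off and reverses to switch on, with its Luminosity track driving the spotlight intensity.
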(event EventBeginPlay
  (|CallParentFunction)
  (Variables|Default|SetisOn? true)
  (bind _luminosity (Timeline|Off Reverse)
    (:Update
      (Rendering|Components|Light|SetIntensity (Variables|Default|GetSpotLight) _luminosity))))

(event EventInteract
  (|CallParentFunction)
  (bind _output_get (Variables|Default|SetisOn? (not (Variables|Default|GetisOn?))))
  (if _output_get
    (bind _luminosity (Timeline|Off Reverse)
      (:Update
        (Rendering|Components|Light|SetIntensity (Variables|Default|GetSpotLight) _luminosity)))
    (else
      (Timeline|Off Play))))

(fn ConstructionScript
  (|CallParentFunction))