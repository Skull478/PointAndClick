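; Interactive phone actor, built on a parent class, that plays call audio and lets an interaction toggle a talking state.
; BeginPlay starts Audio2 and immediately pauses it, so each Interact flips IsTalking and resumes or pauses that track rather than restarting it.
; A separate Call event plays Audio1 from the start, independently of the talking state.
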(event Custom|Call
  (Audio|Components|Audio|Play (Variables|Default|GetAudio%20-%201) 0.0))

(event EventBeginPlay
  (bind _audio___2 (Variables|Default|GetAudio%20-%202))
  (|CallParentFunction)
  (Variables|Default|SetisTalking? false)
  (Audio|Components|Audio|Play _audio___2 0.0)
  (Class|AudioComponent|SetPaused _audio___2 true))

(event EventInteract
  (bind _audio___2 (Variables|Default|GetAudio%20-%202))
  (|CallParentFunction)
  (bind _output_get (Variables|Default|SetisTalking? (not (Variables|Default|GetisTalking?))))
  (if _output_get
    (Class|AudioComponent|SetPaused _audio___2 false)
    (else
      (Class|AudioComponent|SetPaused _audio___2 true))))

(fn ConstructionScript
  (|CallParentFunction))