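; Interactive switch actor, derived from a parent interactive Blueprint, that toggles a glowing mesh and its point light.
; It starts on at BeginPlay, and each Interact flips the state, swapping between glow and no-glow materials.
; The Off timeline drives light intensity, playing forward to switch off and reversing to switch on.
; Two sphere triggers independently show and hide their paired widgets on overlap.
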(event OnComponentBeginOverlap(Sphere)
  (params (OverlappedComponent :type Primitive%20Component%20Object%20Reference) (OtherActor :type Actor%20Object%20Reference) (OtherComp :type Primitive%20Component%20Object%20Reference) (OtherBodyIndex :type Integer) (bFromSweep :type Boolean) (SweepResult :type Hit%20Result%20Structure%20%28by%20ref%29))
  (Rendering|SetVisibility (Variables|Default|GetWidget) true false))

(event OnComponentEndOverlap(Sphere)
  (params (OverlappedComponent :type Primitive%20Component%20Object%20Reference) (OtherActor :type Actor%20Object%20Reference) (OtherComp :type Primitive%20Component%20Object%20Reference) (OtherBodyIndex :type Integer))
  (Rendering|SetVisibility (Variables|Default|GetWidget) false false))

(event OnComponentBeginOverlap(Sphere2)
  (params (OverlappedComponent :type Primitive%20Component%20Object%20Reference) (OtherActor :type Actor%20Object%20Reference) (OtherComp :type Primitive%20Component%20Object%20Reference) (OtherBodyIndex :type Integer) (bFromSweep :type Boolean) (SweepResult :type Hit%20Result%20Structure%20%28by%20ref%29))
  (Rendering|SetVisibility (Variables|Default|GetWidget2) true false))

(event OnComponentEndOverlap(Sphere2)
  (params (OverlappedComponent :type Primitive%20Component%20Object%20Reference) (OtherActor :type Actor%20Object%20Reference) (OtherComp :type Primitive%20Component%20Object%20Reference) (OtherBodyIndex :type Integer))
  (Rendering|SetVisibility (Variables|Default|GetWidget2) false false))

(event EventBeginPlay
  (|CallParentFunction)
  (Variables|Default|SetisOn? true)
  (Rendering|Material|SetMaterial (Variables|Default|GetStaticMesh) 0 "/Game/DetectiveStart/Assets/Materials/M_Glow.M_Glow")
  (bind _luminosity (Timeline|Off Reverse)
    (:Update
      (Rendering|Components|Light|SetIntensity (Variables|Default|GetPointLight) _luminosity))))

(event EventInteract
  (bind _staticmesh (Variables|Default|GetStaticMesh))
  (|CallParentFunction)
  (bind _output_get (Variables|Default|SetisOn? (not (Variables|Default|GetisOn?))))
  (if _output_get
    (Rendering|Material|SetMaterial _staticmesh 0 "/Game/DetectiveStart/Assets/Materials/M_Glow.M_Glow")
    (bind _luminosity (Timeline|Off Reverse)
      (:Update
        (Rendering|Components|Light|SetIntensity (Variables|Default|GetPointLight) _luminosity)))
    (else
      (Rendering|Material|SetMaterial _staticmesh 0 "/Game/DetectiveStart/Assets/Materials/M_NoGlow.M_NoGlow")
      (Timeline|Off Play))))

(fn ConstructionScript
  (|CallParentFunction))