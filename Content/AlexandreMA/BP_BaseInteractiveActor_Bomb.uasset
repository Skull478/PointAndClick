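; Interactive bomb actor that counts as a collectable: interacting removes it, decrements CollectableLeft in FirstPersonGameMode, and opens Map_Win when none remain.
; A Hint timeline pulses its point light, using a FlipFlop to fade forward and back with a random pause between pulses.
; A separate Boom event, not called within this graph, spawns a huge explosion effect and sound, then destroys the actor.
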(event Custom|Boom
  (Effects|SpawnEmitteratLocation "/Game/StarterContent/Particles/P_Explosion.P_Explosion" (Transformation|GetActorLocation) "0, 0, 0" "50.000000,50.000000,50.000000")
  (Audio|PlaySound2D "/Game/StarterContent/Audio/Explosion01.Explosion01" 3.0 1.0 0.0 0 0)
  (Actor|DestroyActor))

(event EventBeginPlay
  (|CallParentFunction)
  (bind _fade (Timeline|Hint PlayFromStart)
    (:Update
      (Rendering|Components|Light|SetIntensity (Variables|Default|GetPointLight) _fade))
    (:Finished
      (Utilities|FlowControl|FlipFlop
        (:A
          (Timeline|Hint ReverseFromEnd))
        (:B
          (Utilities|FlowControl|Delay (Math|Random|RandomFloatinRange 2.0 4.0))
          (Timeline|Hint PlayFromStart))))))

(event EventInteract
  (|CallParentFunction)
  (bind _asfirst_person_game_mode (Utilities|Casting|CastToFirstPersonGameMode (Game|GetGameMode)))
  (bind _result (Math|Integer|DecrementInt (Variables|/Game/FirstPersonGameMode.FirstPersonGameMode_C|GetCollectable_Left _asfirst_person_game_mode))
    (:%20%20
      (Variables|/Game/FirstPersonGameMode.FirstPersonGameMode_C|SetCollectable_Left _asfirst_person_game_mode _result)
      (Actor|DestroyActor)
      (if (== (Variables|/Game/FirstPersonGameMode.FirstPersonGameMode_C|GetCollectable_Left _asfirst_person_game_mode) 0)
        (Game|OpenLevel(byObjectReference) "/Game/Clement_K/Level/Map_Win.Map_Win")))))

(fn ConstructionScript
  (|CallParentFunction))